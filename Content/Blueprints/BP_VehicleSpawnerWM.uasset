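; Vehicle spawner placed in levels, extending a parent spawner, that can pin a specific vehicle through the VehicleToSpawn enum.
; All logic is in the construction script: a non-default choice replaces VehicleIDs, and the parent script runs afterwards, plus earlier when none is chosen.
; The enum name also keys a DTT_VehicleSpawnerWM row that sets the editor preview mesh and label.
; HideInGameView controls whether both are hidden in game.
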(fn `UserConstructionScript`
  (bind _vehicle (`self.Vehicle`))
  (bind _hideingameview (`self.HideInGameView`))
  (`|ExecutionSequence`
    (:`then_0`
      ;[1 1 1] Set Unique Vehicle - Spawn a specific Vehicle
      (if (> (`self.VehicleToSpawn`) 0)
        (`KismetArrayLibrary.Array_Clear` (`self.VehicleIDs`))
        (`KismetArrayLibrary.Array_AddUnique` (`self.VehicleIDs`) (`KismetStringLibrary.Conv_StringToName` (`|GetEnumeratorNameAsString` (`self.VehicleToSpawn`))))
        (else
          (`parent.UserConstructionScript`))))
    (:`then_1`
      ;[1 1 1] Set Visible Editor Model - Set the Visible Model based on last selected Vehicle - Editor Only
      (bind _returnvalue (`|GetDataTableRow` "/Game/Blueprints/DTT_VehicleSpawnerWM.DTT_VehicleSpawnerWM" (`KismetStringLibrary.Conv_StringToName` (`|GetEnumeratorNameAsString` (`self.VehicleToSpawn`))))
        (:`then`
          (`StaticMeshComponent.SetStaticMesh` (`self.Vehicle`) (`.StaticMesh_2_F101FA76442D70DCF4CA41BBABC41738` (break `/Game/Blueprints/STR_SpawnerWM` _returnvalue)))
          (`TextRenderComponent.K2_SetText` (`self.Name`) (`KismetTextLibrary.Conv_NameToText` (break `/Game/Blueprints/STR_SpawnerWM` _returnvalue))))))
    (:`then_2`
      ;[1 1 1] Hide in Game View - Toggle the Visible Model in Game View (G) - Editor Only
      (`/Engine/EditorBlueprintResources/StandardMacros.FlipFlop`
        (:`A`
          (`SceneComponent.SetHiddenInGame` _vehicle _hideingameview false)
          (`SceneComponent.SetHiddenInGame` (`self.Name`) _hideingameview false))
        (:`B`
          (`SceneComponent.SetHiddenInGame` _vehicle _hideingameview false)
          (`SceneComponent.SetHiddenInGame` (`self.Name`) _hideingameview false))))
    (:`then_3`
      (`parent.UserConstructionScript`))))