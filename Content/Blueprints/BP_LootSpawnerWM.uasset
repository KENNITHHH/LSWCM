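; BP_LootSpawnerWM is a placeable loot spawner configured in the editor, with a preview mesh of the chosen item.
; Its construction script turns the LootToSpawn enum into SpawnList entries, either accumulating a random pool or keeping one specific item.
; The last selection keys into DTT_LootSpawnerWM to set the preview mesh, whose in-game visibility follows HideInGameView.
; The event graph is empty, so this file holds no runtime spawning logic.
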(fn `UserConstructionScript`
  (bind _item (`self.Item`))
  (bind _hideingameview (`self.HideInGameView`))
  (`|ExecutionSequence`
    (:`then_0`
      ;[1 1 1] Make Random List - Add multiple items for random item spawn
      (if (`self.MakeRandomList?`)
        (if (> (`self.LootToSpawn`) 0)
          (`KismetArrayLibrary.Array_AddUnique` (`self.SpawnList`) (`|GetEnumeratorNameAsString` (`self.LootToSpawn`)))
          (else
            (`parent.UserConstructionScript`)))
        (else
          ;[1 1 1] Set Unique Item - Spawn a specific item
          (if (> (`self.LootToSpawn`) 0)
            (`KismetArrayLibrary.Array_Clear` (`self.SpawnList`))
            (`KismetArrayLibrary.Array_AddUnique` (`self.SpawnList`) (`|GetEnumeratorNameAsString` (`self.LootToSpawn`)))
            (else
              (`parent.UserConstructionScript`))))))
    (:`then_1`
      ;[1 1 1] Set Visible Editor Model - Set the Visible Model based on last selected Item - Editor Only
      (bind _returnvalue (`|GetDataTableRow` "/Game/Blueprints/DTT_LootSpawnerWM.DTT_LootSpawnerWM" (`KismetStringLibrary.Conv_StringToName` (`|GetEnumeratorNameAsString` (`self.LootToSpawn`))))
        (:`then`
          (`StaticMeshComponent.SetStaticMesh` (`self.Item`) (`.StaticMesh_2_F101FA76442D70DCF4CA41BBABC41738` (break `/Game/Blueprints/STR_SpawnerWM` _returnvalue))))))
    (:`then_2`
      ;[1 1 1] Hide in Game View - Toggle the Visible Model in Game View (G) - Editor Only
      (`/Engine/EditorBlueprintResources/StandardMacros.FlipFlop`
        (:`A`
          (`SceneComponent.SetHiddenInGame` _item _hideingameview false))
        (:`B`
          (`SceneComponent.SetHiddenInGame` _item _hideingameview false))))
    (:`then_3`
      (`parent.UserConstructionScript`))))